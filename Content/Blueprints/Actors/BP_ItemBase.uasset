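; Base actor for clickable sprite items that the player can inspect up close or interact with.
; Shift-click toggles zoom by moving the BP_Camera pawn to the item's zoom point or back to its current room's root, tracked by ItemState.
; A plain click branches on ItemClickActionType to either add the ItemStruct data to a player slot, destroying the actor on success, or call RevealNewItemAndDestroy.
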(event OnBeginCursorOver(PaperSprite)
  (params (TouchedComponent :type Primitive%20Component%20Object%20Reference)))

(event Custom|PerformZoomOperation
  (if (Utilities|Enum|Equal(Enum) (Variables|Default|GetItemState) "NewEnumerator1")
    (CallFunction|ZoomOutObject)
    (else
      (CallFunction|ZoominObject))))

(event Custom|Sprite%20Clicked
  (params (TouchedComponent :type Primitive%20Component%20Object%20Reference) (ButtonPressed :type Key%20Structure :default "None"))
  (if (Variables|/Game/Blueprints/Camera/BP_Camera.BP_Camera_C|GetbIsHoldingShift (Variables|Default|GetPlayer))
    (CallFunction|PerformZoomOperation)
    (else
      (CallFunction|Interact))))

(event EventBeginPlay
  (bind _asbp_camera (Utilities|Casting|CastToBP_Camera (Game|Player|GetPlayerPawn 0)))
  (Variables|Default|SetPlayer _asbp_camera)
  (EventDispatchers|AssignOnClicked (Variables|Default|GetPaperSprite) (delegate Custom|Sprite%20Clicked)))

(event EventInteract
  (switch Utilities|FlowControl|Switch|SwitchonE_ItemClickActionType (Variables|Default|GetItemClickActionType)
    (:NewEnumerator0
      (CallFunction|AddtoInventory))
    (:NewEnumerator1
      (CallFunction|RevealNewItemandDestroy))))

(event EventAddtoInventory
  (bind _itemstruct (Variables|Default|GetItemStruct))
  (bind (_slotid _itemid _itemname _itemdescription _itemicon _taskid) (Utilities|Struct|BreakS_ItemStruct _itemstruct))
  ;[1 1 1] Add To Inventory Base Logic
  (bind _found_slot (Default|AddtoSlot (Variables|Default|GetPlayer) _itemid _itemname _itemdescription _itemicon _taskid))
  (if _found_slot
    (Development|PrintString "Item Added")
    (Actor|DestroyActor)
    (else
      (Development|PrintString "Item Not Added" true true "(R=1.000000,G=0.071010,B=0.000000,A=1.000000)"))))

(fn ConstructionScript)

(fn ZoominObject
  (if (Utilities|Enum|NotEqual(Enum) (Variables|Default|GetItemState) "NewEnumerator1")
    (bind _asbp_camera (Utilities|Casting|CastToBP_Camera (Game|Player|GetPlayerPawn 0)))
    (Transformation|SetActorLocation _asbp_camera (Transformation|GetWorldLocation (Variables|Default|GetCameraZoomedInPosition)) false false)
    (Variables|Default|SetItemState "NewEnumerator1")
    (else
      (Development|PrintString "Fail"))))

(fn ZoomOutObject
  (if (Utilities|Enum|Equal(Enum) (Variables|Default|GetItemState) "NewEnumerator1")
    (bind _asbp_camera (Utilities|Casting|CastToBP_Camera (Game|Player|GetPlayerPawn 0)))
    (Transformation|SetActorLocation _asbp_camera (Transformation|GetWorldLocation (Variables|/Game/Blueprints/Actors/BP_CameraMovePoint.BP_CameraMovePoint_C|GetDefaultSceneRoot (.Value (Utilities|Map|Find (Variables|/Game/Blueprints/Camera/BP_Camera.BP_Camera_C|GetRooms _asbp_camera) (Variables|/Game/Blueprints/Camera/BP_Camera.BP_Camera_C|GetCurrentRoomId _asbp_camera))))) false false)
    (Variables|Default|SetItemState "NewEnumerator0")))