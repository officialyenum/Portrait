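; BP_VanityTable is an interactable Level 3 vanity table with clickable boxes for a first drawer, magnet drawer and eye shadow, still at stub stage.
; Interact and the three OnClicked events only print debug strings and call none of the open functions.
; OpenFirstDrawer switches on a combined DrawerState enum, but every listed state prints the same "closed" message.
; OpenMagnetDrawer and OpenEyeShadow are empty, and GrabItem's switch on ItemId has no cases.
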(event OnClicked(FirstDrawerBox)
  (params (TouchedComponent :type Primitive%20Component%20Object%20Reference) (ButtonPressed :type Key%20Structure))
  (Development|PrintString "FirstDrawerClicked"))

(event OnClicked(MagnetDrawerBox)
  (params (TouchedComponent :type Primitive%20Component%20Object%20Reference) (ButtonPressed :type Key%20Structure))
  (Development|PrintString "MagnetClicked"))

(event OnClicked(EyeShadowBox)
  (params (TouchedComponent :type Primitive%20Component%20Object%20Reference) (ButtonPressed :type Key%20Structure))
  (Development|PrintString "EyeShadowClicked"))

(event EventBeginPlay
  (|CallParentFunction) ; This node is disabled and will not be called.\nDrag off pins to build functionality.
)

(event Collision|EventActorBeginOverlap
  (params (OtherActor :type Actor%20Object%20Reference))
  (|CallParentFunction OtherActor) ; This node is disabled and will not be called.\nDrag off pins to build functionality.
)

(event EventTick
  (params (DeltaSeconds :type Float%20%28single-precision%29))
  (|CallParentFunction DeltaSeconds) ; This node is disabled and will not be called.\nDrag off pins to build functionality.
)

(event EventInteract
  (|CallParentFunction)
  (Development|PrintString "Interacting with Event"))

(fn ConstructionScript
  (|CallParentFunction))

(fn OpenFirstDrawer
  (switch Utilities|FlowControl|Switch|SwitchonE_DrawerState (Variables|Default|GetDrawerState)
    (:NewEnumerator0
      _)
    (:NewEnumerator1
      _)
    (:NewEnumerator4
      _)
    (:NewEnumerator5
      _)
    (:NewEnumerator8
      _)
    (:NewEnumerator9
      _))
  (Development|PrintString "Drawer is currently closed"))

(fn OpenMagnetDrawer)

(fn OpenEyeShadow)

(fn GrabItem
  (params (itemId :type Integer))
  (switch int itemId))