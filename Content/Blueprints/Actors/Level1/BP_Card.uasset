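; BP_Card is an interactable card actor for Level 1 that can be replaced by another item.
; BeginPlay, Interact and construction only call the parent class.
; Its reveal event spawns the configured item class at the card's transform, passes it an item struct, calls ShowImageInUI and destroys the card.
; An invalid class prints an error message and leaves the card in place.
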(event EventBeginPlay
  (|CallParentFunction))

(event EventRevealNewItemandDestroy
  (if (Utilities|IsValidClass (Variables|Default|GetSpawnableItemClass))
    (Game|SpawnActorfromClass :Class (Variables|Default|GetSpawnableItemClass) :SpawnTransform (Transformation|GetActorTransform) :CollisionHandlingOverride "Undefined" :TransformScaleMethod "MultiplyWithRoot" :ItemStruct (Variables|Default|GetSpawnableItemStruct) :SpawnableItemClass 0 :Instigator 0)
    (CallFunction|ShowImageinUI)
    (Actor|DestroyActor)
    (else
      (Development|PrintString "Invalid Class" true true "(R=1.000000,G=0.071010,B=0.000000,A=1.000000)"))))

(event EventInteract
  (|CallParentFunction))

(fn ConstructionScript
  (|CallParentFunction))