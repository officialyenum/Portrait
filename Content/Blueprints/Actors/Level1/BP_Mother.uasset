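; BP_Mother is an interactable Level 1 actor for the mother character that shows dialogue when the player interacts with it.
; Interact plays a 2D click sound, then calls ShowDialogue, which makes a dialogue sprite visible and hides it again after a four-second delay.
; BeginPlay and the construction script add no logic of their own.
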(event EventBeginPlay
  (|CallParentFunction) ; This node is disabled and will not be called.\nDrag off pins to build functionality.
)

(event EventInteract
  (Audio|PlaySound2D (Variables|Default|GetObjectClickSound) 1.0 1.0 0.0 0 0)
  (CallFunction|ShowDialogue))

(event EventShowDialogue
  (bind _dialoguesprite (Variables|Default|GetDialogueSprite))
  (Rendering|SetVisibility _dialoguesprite true false)
  (Utilities|FlowControl|Delay 4.0)
  (Rendering|SetVisibility _dialoguesprite false false))

(fn ConstructionScript
  (|CallParentFunction))