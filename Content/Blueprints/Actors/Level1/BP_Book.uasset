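; BP_Book is a Level 1 book actor that, when revealed, replaces itself with a new item.
; Interact defers to the parent class, while RevealNewItemandDestroy spawns SpawnableItemClass at the book's transform using SpawnableItemStruct, then shows a UI image and destroys the book.
; The spawned actor receives BP_Note and the "Note For Maddie" item data as its own next spawnable item, chaining the reveals.
; An invalid class only prints an error.
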(event EventBeginPlay
  (|CallParentFunction) ; This node is disabled and will not be called.\nDrag off pins to build functionality.
)

(event Collision|EventActorBeginOverlap
  (params (OtherActor :type Actor%20Object%20Reference))
  (|CallParentFunction OtherActor) ; This node is disabled and will not be called.\nDrag off pins to build functionality.
)

(event EventTick
  (params (DeltaSeconds :type Float%20%28single-precision%29))
  (|CallParentFunction DeltaSeconds) ; This node is disabled and will not be called.\nDrag off pins to build functionality.
)

(event EventInteract
  (|CallParentFunction))

(event EventRevealNewItemandDestroy
  (bind _spawnableitemclass (Variables|Default|GetSpawnableItemClass))
  (if (Utilities|IsValidClass _spawnableitemclass)
    (Game|SpawnActorfromClass _spawnableitemclass (Transformation|GetActorTransform) "AlwaysSpawn" "MultiplyWithRoot" 0 "NewEnumerator0" (Variables|Default|GetSpawnableItemStruct) "/Game/Blueprints/Actors/Level1/BP_Note.BP_Note_C" (Utilities|Struct|MakeS_ItemStruct 0 6 "Note" "Note For Maddie" "/Game/Assets/Textures/UI/Ui_icon_Note.Ui_icon_Note" 2 true) 0)
    (CallFunction|ShowImageinUI)
    (Actor|DestroyActor)
    (else
      (Development|PrintString "Invalid Class" true true "(R=1.000000,G=0.071010,B=0.000000,A=1.000000)"))))

(fn ConstructionScript
  (|CallParentFunction))