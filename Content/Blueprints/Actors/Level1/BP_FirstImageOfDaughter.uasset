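; BP_FirstImageOfDaughter is an interactable Level 1 actor, the daughter's first image, that ends play by switching the menu to Credits.
; On Interact, if it is not hidden, it plays a 2D click sound and calls GoToNextLevel.
; Despite its name, GoToNextLevel loads no level, instead casting to BP_PlayerController and updating the menu through its HUD.
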(event EventBeginPlay
  (|CallParentFunction) ; This node is disabled and will not be called.\nDrag off pins to build functionality.
)

(event EventGotoNextLevel
  (bind _asbp_player_controller (Utilities|Casting|CastToBP_PlayerController (Game|GetPlayerController 0)))
  (Default|UpdateMenu (Variables|/Game/Blueprints/Controller/BP_PlayerController.BP_PlayerController_C|GetBP%20Hud _asbp_player_controller) "Credits"))

(event EventInteract
  (if (not (Variables|Default|GetbHidden))
    (Audio|PlaySound2D (Variables|Default|GetObjectClickSound) 1.0 1.0 0.0 0 0)
    (CallFunction|GotoNextLevel)))

(fn ConstructionScript
  (|CallParentFunction))