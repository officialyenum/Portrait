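; Player controller that turns Enhanced Input actions into camera level navigation, pause and quit.
; On BeginPlay it adds the portrait mapping context and caches BP_Hud.
; Next/previous actions move the BP_Camera pawn between levels and refresh the game HUD's task list, while Shift sets a hold flag on that pawn.
; Pause toggles the game's paused state and switches the HUD between Pause and Game menus; Quit exits the game.
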(event Custom|UpdateUITaskList
  (bind _aswbp_game_hud (Utilities|Casting|CastToWBP_GameHud (Variables|/Game/Blueprints/UI/BP_Hud.BP_Hud_C|GetCurrentWidget (Variables|Default|GetBP%20Hud))))
  (Default|UpdateTaskList (Variables|/Game/Blueprints/UI/UserWidgets/WBP_GameHud.WBP_GameHud_C|GetWBP_TaskListView _aswbp_game_hud)))

(event Custom|PauseLogic
  (if (not (Variables|Default|GetbGameIsPaused))
    (Game|SetGamePaused true)
    (Default|UpdateMenu (Variables|Default|GetBP%20Hud) "Pause")
    (Variables|Default|SetbGameIsPaused true)
    (else
      (Game|SetGamePaused false)
      (Default|UpdateMenu (Variables|Default|GetBP%20Hud) "Game")
      (Variables|Default|SetbGameIsPaused false))))

(event Custom|QuitGameLogic
  (Game|QuitGame self "Quit" false))

(event Input|EnhancedActionEvents|EnhancedInputActionIA_CameraNext
  (params (ActionValue :type Boolean) (ElapsedSeconds :type Float%20%28double-precision%29) (TriggeredSeconds :type Float%20%28double-precision%29) (InputAction :type Input%20Action%20Object%20Reference :default "/Game/Inputs/Actions/IA_CameraNext.IA_CameraNext"))
  (:Started
    (Development|PrintString "Move Camera To Next Location")
    (bind _asbp_camera (Utilities|Casting|CastToBP_Camera (Game|Player|GetPlayerPawn 0)))
    (Default|GotoNextLevel _asbp_camera)
    (CallFunction|UpdateUITaskList)))

(event Input|EnhancedActionEvents|EnhancedInputActionIA_CameraPrev
  (params (ActionValue :type Boolean) (ElapsedSeconds :type Float%20%28double-precision%29) (TriggeredSeconds :type Float%20%28double-precision%29) (InputAction :type Input%20Action%20Object%20Reference :default "/Game/Inputs/Actions/IA_CameraPrev.IA_CameraPrev"))
  (:Started
    (Development|PrintString "Move Camera To Previous Location")
    (bind _asbp_camera (Utilities|Casting|CastToBP_Camera (Game|Player|GetPlayerPawn 0)))
    (Default|GotoPreviousLevel _asbp_camera)
    (CallFunction|UpdateUITaskList)))

(event Input|EnhancedActionEvents|EnhancedInputActionIA_Shift
  (params (ActionValue :type Boolean) (ElapsedSeconds :type Float%20%28double-precision%29) (TriggeredSeconds :type Float%20%28double-precision%29) (InputAction :type Input%20Action%20Object%20Reference :default "/Game/Inputs/Actions/IA_Shift.IA_Shift"))
  (:Triggered
    (bind _asbp_camera (Utilities|Casting|CastToBP_Camera (Game|Player|GetPlayerPawn 0) :!label _label))
    (Variables|/Game/Blueprints/Camera/BP_Camera.BP_Camera_C|SetbIsHoldingShift _asbp_camera true))
  (:Started
    (goto _label))
  (:Completed
    (bind _asbp_camera_2 (Utilities|Casting|CastToBP_Camera (Game|Player|GetPlayerPawn 0)))
    (Variables|/Game/Blueprints/Camera/BP_Camera.BP_Camera_C|SetbIsHoldingShift _asbp_camera_2 false)))

(event Input|EnhancedActionEvents|EnhancedInputActionIA_Pause
  (params (ActionValue :type Boolean) (ElapsedSeconds :type Float%20%28double-precision%29) (TriggeredSeconds :type Float%20%28double-precision%29) (InputAction :type Input%20Action%20Object%20Reference :default "/Game/Inputs/Actions/IA_Pause.IA_Pause"))
  (:Started
    (CallFunction|PauseLogic)))

(event Input|EnhancedActionEvents|EnhancedInputActionIA_Quit
  (params (ActionValue :type Boolean) (ElapsedSeconds :type Float%20%28double-precision%29) (TriggeredSeconds :type Float%20%28double-precision%29) (InputAction :type Input%20Action%20Object%20Reference :default "/Game/Inputs/Actions/IA_Quit.IA_Quit"))
  (:Started
    (CallFunction|QuitGameLogic)))

(event EventBeginPlay
  (Input|AddMappingContext (PlayerController|LocalPlayerSubsystems|GetEnhancedInputLocalPlayerSubsystem) "/Game/Inputs/IMC_Portrait.IMC_Portrait" 0 "(bIgnoreAllPressedKeysUntilRelease=True,bForceImmediately=False,bNotifyUserSettings=False)")
  (bind _asbp_hud (Utilities|Casting|CastToBP_Hud (HUD|GetHUD)))
  (Variables|Default|SetBP%20Hud _asbp_hud))

(event EventTick
  (params (DeltaSeconds :type Float%20%28single-precision%29)))

(fn ConstructionScript)