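; Camera actor that teleports between rooms by ID and holds the game's item inventory and task state.
; Slot and task maps are edited through add, remove and update functions, with changes announced through update calls.
; Tasks complete only in their own room; finishing a room's tasks unhides a daughter image via the GameMode.
; Events reach the HUD widget to refresh inventory or showcase images, while the task-list event stops after its cast.
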(event Custom|UpdateGameHud
  (bind _asbp_player_controller (Utilities|Casting|CastToBP_PlayerController (Game|GetPlayerController 0)))
  (bind _asbp_hud (Utilities|Casting|CastToBP_Hud (HUD|GetHUD _asbp_player_controller)))
  (bind _aswbp_game_hud (Utilities|Casting|CastToWBP_GameHud (Variables|/Game/Blueprints/UI/BP_Hud.BP_Hud_C|GetCurrentWidget _asbp_hud)))
  (Default|UpdateInventory _aswbp_game_hud))

(event Custom|Show%20Image%20In%20UI
  (params (Image :type Object%20Object%20Reference))
  (bind _asbp_player_controller (Utilities|Casting|CastToBP_PlayerController (Game|GetPlayerController 0)))
  (bind _asbp_hud (Utilities|Casting|CastToBP_Hud (HUD|GetHUD _asbp_player_controller)))
  (bind _aswbp_game_hud (Utilities|Casting|CastToWBP_GameHud (Variables|/Game/Blueprints/UI/BP_Hud.BP_Hud_C|GetCurrentWidget _asbp_hud)))
  (Default|ShowcaseImageEvent _aswbp_game_hud Image))

(event Custom|UpdateTaskList
  (bind _asbp_player_controller (Utilities|Casting|CastToBP_PlayerController (Game|GetPlayerController 0)))
  (bind _asbp_hud (Utilities|Casting|CastToBP_Hud (HUD|GetHUD _asbp_player_controller)))
  (Utilities|Casting|CastToWBP_GameHud (Variables|/Game/Blueprints/UI/BP_Hud.BP_Hud_C|GetCurrentWidget _asbp_hud)))

(event EventBeginPlay)

(event Collision|EventActorBeginOverlap
  (params (OtherActor :type Actor%20Object%20Reference)))

(event EventTick
  (params (DeltaSeconds :type Float%20%28single-precision%29)))

(fn ConstructionScript)

(fn GotoNextLevel
  (bind _currentroomid (Variables|Default|GetCurrentRoomId))
  (if (<= _currentroomid 2)
    (bind _result (Math|Integer|IncrementInt _currentroomid)
      (:%20%20
        (if (.ReturnValue (Utilities|Map|Find (Variables|Default|GetRooms) _result))
          (Transformation|SetActorLocation self (Transformation|GetWorldLocation (Variables|/Game/Blueprints/Actors/BP_CameraMovePoint.BP_CameraMovePoint_C|GetDefaultSceneRoot (.Value (Utilities|Map|Find (Variables|Default|GetRooms) _result)))) false true)
          (else
            (Development|PrintString "Room Not Found" true true "(R=1.000000,G=0.071010,B=0.000000,A=1.000000)")))))
    (else
      (Development|PrintString "Current Room Id is LESS OR EQUAL 2" true true "(R=1.000000,G=0.071010,B=0.000000,A=1.000000)"))))

(fn GotoPreviousLevel
  (bind _currentroomid (Variables|Default|GetCurrentRoomId))
  (if (>= _currentroomid 2)
    (bind _result (Math|Integer|DecrementInt _currentroomid)
      (:%20%20
        (Development|PrintString "Hello" (.ReturnValue (Utilities|Map|Find (Variables|Default|GetRooms) _result)))
        (Transformation|SetActorLocation self (Transformation|GetWorldLocation (Variables|/Game/Blueprints/Actors/BP_CameraMovePoint.BP_CameraMovePoint_C|GetDefaultSceneRoot (.Value (Utilities|Map|Find (Variables|Default|GetRooms) _result)))) false true)))
    (else
      (Development|PrintString "Current Room Id IS Greater OR Equal to 2"))))

(fn AddtoSlot
  (params (ItemId :type Integer) (ItemName :type String) (ItemDescription :type String) (ItemIcon :type Texture%20Object%20Reference) (TaskId :type Integer))
  (bind _slotinventory (Variables|Default|GetSlotInventory))
  (bind _values (Utilities|Map|Values _slotinventory))
  (for _array_element _values
    (if (not (.bIsOccupied (Utilities|Struct|BreakS_ItemStruct _array_element)))
      (Utilities|Map|Add _slotinventory (.SlotId (Utilities|Struct|BreakS_ItemStruct _array_element)) (Utilities|Struct|MakeS_ItemStruct (.SlotId (Utilities|Struct|BreakS_ItemStruct _array_element)) ItemId ItemName ItemDescription ItemIcon TaskId true))
      (Default|CallOnSlotUpdated (Variables|Default|GetSlotInventory))
      (return true)))
  (return false))

(fn UpdateTask
  (params (Task%20To%20Update%20Id :type Integer))
  (bind _taskinventory (Variables|Default|GetTaskInventory))
  (bind _values (Utilities|Map|Values _taskinventory))
  (for _array_element _values
    (if (== Task%20To%20Update%20Id (.TaskId (Utilities|Struct|BreakS_TaskStruct _array_element)))
      (if (== (Variables|Default|GetCurrentRoomId) (.TaskRoomId (Utilities|Struct|BreakS_TaskStruct _array_element)))
        (Utilities|Map|Add _taskinventory (.TaskId (Utilities|Struct|BreakS_TaskStruct _array_element)) (Utilities|Struct|MakeS_TaskStruct (.TaskName (Utilities|Struct|BreakS_TaskStruct _array_element)) true (.TaskId (Utilities|Struct|BreakS_TaskStruct _array_element)) (.TaskRoomId (Utilities|Struct|BreakS_TaskStruct _array_element))))
        (Default|CallOnTaskUpdated (Variables|Default|GetTaskInventory))
        (bind _biscomplete (CallFunction|CheckTaskCompletebyLevel (.TaskRoomId (Utilities|Struct|BreakS_TaskStruct _array_element))))
        (if _biscomplete
          (bind _asbp_game_mode (Utilities|Casting|CastToBP_GameMode (Game|GetGameMode)))
          (Rendering|SetActorHiddenInGame (Variables|/Game/Blueprints/Game/BP_GameMode.BP_GameMode_C|GetDaughterImageOne _asbp_game_mode) false)
          (return true)
          (else
            (return true)))
        (else
          (Development|PrintString "Wrong Room")
          (return false)))))
  (return false))

(fn RemovefromSlot
  (params (ItemToRemoveId :type Integer))
  (bind _slotinventory (Variables|Default|GetSlotInventory))
  (bind _values (Utilities|Map|Values _slotinventory))
  (for _array_element _values
    (if (== ItemToRemoveId (.ItemId (Utilities|Struct|BreakS_ItemStruct _array_element)))
      (Utilities|Map|Add _slotinventory (.SlotId (Utilities|Struct|BreakS_ItemStruct _array_element)) (Utilities|Struct|MakeS_ItemStruct (.SlotId (Utilities|Struct|BreakS_ItemStruct _array_element)) 0 "" "" "/Game/Assets/Textures/UI/Inventory_Icon.Inventory_Icon"))
      (Default|CallOnSlotUpdated (Variables|Default|GetSlotInventory))
      (return true)))
  (return true))

(fn GetIteminSlot
  (params (Slot%20Id :type Integer%20%28by%20ref%29))
  (bind _slotinventory (Variables|Default|GetSlotInventory))
  (bind (_value _returnvalue) (Utilities|Map|Find _slotinventory Slot%20Id))
  (if _returnvalue
    (return _value)
    (else
      (return ""))))

(fn GetTaskListbyLevel
  (Utilities|Array|Clear (LocalVariables|GetTaskListInCurrentRoom))
  (bind _values (Utilities|Map|Values (Variables|Default|GetTaskInventory)))
  (for _array_element _values
    (if (== (Variables|Default|GetCurrentRoomId) (.TaskRoomId (Utilities|Struct|BreakS_TaskStruct _array_element)))
      (Utilities|Array|Add (LocalVariables|GetTaskListInCurrentRoom) _array_element)))
  (return (LocalVariables|GetTaskListInCurrentRoom)))

(fn CheckTaskCompletebyLevel
  (params (LevelId :type Integer))
  (bind _values (Utilities|Map|Values (Variables|Default|GetTaskInventory)))
  (for _array_element _values
    (if (== LevelId (.TaskRoomId (Utilities|Struct|BreakS_TaskStruct _array_element)))
      (Utilities|Array|Add (LocalVariables|GetTaskForLevel) _array_element)))
  (for _array_element_2 (LocalVariables|GetTaskForLevel)
    (if (not (.TaskStatus (Utilities|Struct|BreakS_TaskStruct _array_element_2)))
      (return false)))
  (return true))

(fn CheckGameComplete
  (for _index (range 1 3)
    (bind _biscomplete (CallFunction|CheckTaskCompletebyLevel _index))
    (if (not _biscomplete)
      (return false)))
  (return true))